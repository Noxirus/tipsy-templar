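; BP_TipsyCharacter is the player character, with Enhanced Input movement relative to an assigned GameCamera and a montage attack.
; The Breadpon weapon attaches to the left hand, with toggleable collision that only prints overlapped actors.
; Holding interact box-traces for a BPI_Interactable, and releasing stops it.
; Pickup and drop functions drive the Hands grab, whose target follows InteractionArea each tick.
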(event `self.ReceivePossessed`
  (params (NewController :type "Controller Object Reference"))
  (`self.SetupInput`)
  (`PrimitiveComponent.SetCollisionEnabled` (`self.BreadCollision`) "NoCollision"))

(event `self.ReceiveTick`
  (params (DeltaSeconds :type "Float (single-precision)"))
  (`self.HoldObject`))

(event `self.BreadCollision.OnComponentBeginOverlap`
  (params (OverlappedComponent :type "PrimitiveComponent Object Reference") (OtherActor :type "Actor Object Reference") (OtherComp :type "PrimitiveComponent Object Reference") (OtherBodyIndex :type Integer) (bFromSweep :type Boolean) (SweepResult :type "HitResult Structure (by ref)"))
  (`KismetSystemLibrary.PrintString` (`KismetStringLibrary.Concat_StrStr` "Hit: " (`KismetSystemLibrary.GetDisplayName` OtherActor))))

(event `EnhancedInput|/Game/TipsyTemplar/Input/IA_Movement`
  (params (ActionValue :type "Vector2D Structure") (ElapsedSeconds :type "Float (double-precision)") (TriggeredSeconds :type "Float (double-precision)") (InputAction :type "InputAction Object Reference" :default "/Game/TipsyTemplar/Input/IA_Movement.IA_Movement"))
  (:`Triggered`
    (`self.AddMovementInput` (`self.GetActorRightVector` (`self.GameCamera`)) ActionValue_X)
    (`self.AddMovementInput` (`self.CameraForward`) ActionValue_Y)))

(event `EnhancedInput|/Game/TipsyTemplar/Input/IA_Attack`
  (params (ActionValue :type Boolean) (ElapsedSeconds :type "Float (double-precision)") (TriggeredSeconds :type "Float (double-precision)") (InputAction :type "InputAction Object Reference" :default "/Game/TipsyTemplar/Input/IA_Attack.IA_Attack"))
  (:`Started`
    (`|PlayMontage` (`self.Mesh`) "/Game/TipsyTemplar/Animations/TipsyTemplar/AM_Attack.AM_Attack")))

(event `EnhancedInput|/Game/TipsyTemplar/Input/IA_Interact`
  (params (ActionValue :type Boolean) (ElapsedSeconds :type "Float (double-precision)") (TriggeredSeconds :type "Float (double-precision)") (InputAction :type "InputAction Object Reference" :default "/Game/TipsyTemplar/Input/IA_Interact.IA_Interact"))
  (:`Started`
    (`self.InteractCheck`))
  (:`Completed`
    (`self.StopInteraction`)))

(fn `AssignCamera`
  (params (GameCamera :type "CameraActor Object Reference"))
  (set `self.GameCamera` GameCamera))

(fn `CameraForward`
  (returns (ReturnValue :type "Vector Structure"))
  (return (`KismetMathLibrary.Vector_Normal2D` (`self.GetActorForwardVector` (`self.GameCamera`)))))

(fn `DropObject`
  (`PhysicsHandleComponent.ReleaseComponent` (`self.Hands`)))

(fn `HoldObject`
  (`/Engine/EditorBlueprintResources/StandardMacros.IsValid` (`PhysicsHandleComponent.GetGrabbedComponent` (`self.Hands`))
    (:`Is Valid`
      (`PhysicsHandleComponent.SetTargetLocation` (`self.Hands`) (`SceneComponent.K2_GetComponentLocation` (`self.InteractionArea`))))))

(fn `InteractCheck`
  (bind _returnvalue (`SceneComponent.K2_GetComponentLocation` (`self.InteractionArea`)))
  (bind _outhits (`KismetSystemLibrary.BoxTraceMulti` :`Start` _returnvalue :`End` _returnvalue :`HalfSize` (`BoxComponent.GetScaledBoxExtent` (`self.InteractionArea`)) :`TraceChannel` "TraceTypeQuery1" :`DrawDebugType` "ForDuration"))
  (for _array_element _outhits
    (bind _asbpi_interactable (cast `/Game/TipsyTemplar/Code/BPI_Interactable` (`.HitActor` (`GameplayStatics.BreakHitResult` _array_element))))
    (if (not (`KismetSystemLibrary.IsValidInterface` (`self.InteractionItem`)))
      (bind _output_get (set `self.InteractionItem` _asbpi_interactable))
      (`/Game/TipsyTemplar/Code/BPI_Interactable.Interact` _output_get self))))

(fn `Math`
  (params (A :type "Float (double-precision)") (B :type "Float (double-precision)") (ClampCeil :type "Float (double-precision)"))
  (returns (Result :type "Float (double-precision)"))
  (return (* (`KismetMathLibrary.FClamp` (+ A B) 0.0 ClampCeil) 2.0)))

(fn `PickupObject`
  (params (Component :type "PrimitiveComponent Object Reference"))
  (`PhysicsHandleComponent.GrabComponentAtLocation` (`self.Hands`) Component "None" (`SceneComponent.K2_GetComponentLocation` (`self.InteractionArea`))))

(fn `SetupInput`
  (bind _asplayer_controller (cast `PlayerController` (`self.GetController`)))
  (`EnhancedInputSubsystemInterface.AddMappingContext` (pcsubsystem `EnhancedInputLocalPlayerSubsystem` _asplayer_controller) "/Game/TipsyTemplar/Input/IMC_Default.IMC_Default" 0 (struct)))

(fn `SetWeaponCollision`
  (params (CollisionResponse :type "ECollisionEnabled Enum" :default "NoCollision"))
  (`PrimitiveComponent.SetCollisionEnabled` (`self.BreadCollision`) CollisionResponse))

(fn `StopInteraction`
  (if (`KismetSystemLibrary.IsValidInterface` (`self.InteractionItem`))
    (`/Game/TipsyTemplar/Code/BPI_Interactable.StopInteract` (`self.InteractionItem`) self)
    (set `self.InteractionItem` null)))

(fn `UserConstructionScript`
  (`SceneComponent.K2_AttachToComponent` (`self.Breadpon`) (`self.Mesh`) "LeftHandSocket" "KeepRelative" "KeepRelative" "KeepRelative" true))