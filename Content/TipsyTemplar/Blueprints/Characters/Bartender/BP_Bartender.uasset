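; Bartender enemy character that hands the player to its AI controller as a target when it sees them.
; BeginPlay caches the player and its AIC_Bartender controller, and PawnSensing's OnSeePawn calls SetTarget on that controller for any BP_TipsyCharacter spotted.
; An unconnected distance-based aggro and escape check, along with dot, cross and direction debug helpers, remains in the graph but never runs, so nothing here clears the target.
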(event `self.ReceiveBeginPlay`
  (bind _returnvalue (`GameplayStatics.GetActorOfClass` "/Game/TipsyTemplar/Blueprints/Characters/Templar/BP_TipsyCharacter.BP_TipsyCharacter_C"))
  (set `self.PlayerReference` _returnvalue)
  (bind _asaic_bartender (cast `/Game/TipsyTemplar/Blueprints/Characters/Bartender/AI/AIC_Bartender` (`self.GetController`)))
  (set `self.AIController` _asaic_bartender))

(event `self.ReceiveTick`
  (params (DeltaSeconds :type "Float (single-precision)")))

(event `self.PawnSensing.OnSeePawn`
  (params (Pawn :type "Pawn Object Reference"))
  (bind _asbp_tipsy_character (cast `/Game/TipsyTemplar/Blueprints/Characters/Templar/BP_TipsyCharacter` Pawn))
  (`/Game/TipsyTemplar/Blueprints/Characters/Bartender/AI/AIC_Bartender.SetTarget` (`self.AIController`) _asbp_tipsy_character))

(fn `CrossProduct`
  (`KismetSystemLibrary.DrawDebugArrow` (`self.K2_GetActorLocation`) (+ (* (`KismetMathLibrary.Cross_VectorVector` (`self.GetActorForwardVector`) (`self.GetActorForwardVector` (`self.PlayerReference`))) 250.0) (`self.K2_GetActorLocation`)) 50.0 (struct :`R` 0.947033 :`G` 1.0 :`A` 1.0) 0.0 5.0))

(fn `DistanceToPlayer`
  (returns (ReturnValue :type "Float (double-precision)"))
  (return (`KismetMathLibrary.Vector_Distance` (`self.K2_GetActorLocation`) (`self.K2_GetActorLocation` (`self.PlayerReference`)))))

(fn `DotProduct`
  (`KismetSystemLibrary.PrintString` (`KismetStringLibrary.Conv_DoubleToString` (`KismetMathLibrary.Dot_VectorVector` (`self.GetActorForwardVector`) (`self.GetActorForwardVector` (`self.PlayerReference`)))) true true (struct :`G` 0.66 :`B` 1.0 :`A` 1.0) 2.0 "Dot"))

(fn `GetVectorToPlayer`
  (`KismetSystemLibrary.DrawDebugArrow` (`self.K2_GetActorLocation`) (+ (* (`KismetMathLibrary.Normal` (- (`self.K2_GetActorLocation` (`self.PlayerReference`)) (`self.K2_GetActorLocation`))) 250.0) (`self.K2_GetActorLocation`)) 50.0 (struct :`R` 1.0 :`B` 0.170282 :`A` 1.0) 0.0 5.0))

(fn `PlayerDotDirection`
  (returns (ReturnValue :type "Float (double-precision)"))
  (return (`KismetMathLibrary.Dot_VectorVector` (`KismetMathLibrary.Normal` (- (`self.K2_GetActorLocation` (`self.PlayerReference`)) (`self.K2_GetActorLocation`))) (`self.GetActorForwardVector`))))

(fn `UserConstructionScript`)