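; BP_TipsyCharacter is a player character Blueprint that moves relative to a camera actor found in the level.
; BeginPlay registers the default Enhanced Input mapping context and caches the first CameraActor found.
; Movement input follows the camera's right vector and its forward vector, flattened and normalized to 2D.
; The jump action does not jump yet; it only prints press, release and held-frame-count debug messages.
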(event `self.ReceiveBeginPlay`
  (`self.SetupInput`)
  (bind _returnvalue (`GameplayStatics.GetActorOfClass` "/Script/Engine.CameraActor"))
  (set `self.GameCamera` _returnvalue))

(event `EnhancedInput|/Game/TipsyTemplar/Input/IA_Jump`
  (params (ActionValue :type Boolean) (ElapsedSeconds :type "Float (double-precision)") (TriggeredSeconds :type "Float (double-precision)") (InputAction :type "InputAction Object Reference" :default "/Game/TipsyTemplar/Input/IA_Jump.IA_Jump"))
  (:`Triggered`
    (bind _result (`/Engine/EditorBlueprintResources/StandardMacros.IncrementInt` (`self.FrameCount`))
      (:`  `
        (`KismetSystemLibrary.PrintString` (`KismetStringLibrary.Concat_StrStr` "Frame Count: " (`KismetStringLibrary.Conv_IntToString` _result)) true true (struct :`R` 1.0 :`B` 0.087231 :`A` 1.0) 0.0 "2"))))
  (:`Started`
    (set `self.FrameCount` 0)
    (`KismetSystemLibrary.PrintString` "Started Pressing" true true (struct :`G` 1.0 :`B` 0.199344 :`A` 1.0) 5.0 "1"))
  (:`Completed`
    (`KismetSystemLibrary.PrintString` "Finished Pressing" true true (struct :`R` 1.0 :`B` 0.960002 :`A` 1.0) 5.0)))

(event `EnhancedInput|/Game/TipsyTemplar/Input/IA_Movement`
  (params (ActionValue :type "Vector2D Structure") (ElapsedSeconds :type "Float (double-precision)") (TriggeredSeconds :type "Float (double-precision)") (InputAction :type "InputAction Object Reference" :default "/Game/TipsyTemplar/Input/IA_Movement.IA_Movement"))
  (:`Triggered`
    (`self.AddMovementInput` (`self.GetActorRightVector` (`self.GameCamera`)) ActionValue_X)
    (`self.AddMovementInput` (`self.CameraForward`) ActionValue_Y)))

(fn `CameraForward`
  (returns (ReturnValue :type "Vector Structure"))
  (return (`KismetMathLibrary.Vector_Normal2D` (`self.GetActorForwardVector` (`self.GameCamera`)))))

(fn `SetupInput`
  (bind _asplayer_controller (cast `PlayerController` (`self.GetController`)))
  (`EnhancedInputSubsystemInterface.AddMappingContext` (pcsubsystem `EnhancedInputLocalPlayerSubsystem` _asplayer_controller) "/Game/TipsyTemplar/Input/IMC_Default.IMC_Default" 0 (struct)))

(fn `UserConstructionScript`)