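; BP_TipsyGameMode is the Tipsy Templar game mode that sets up the follow camera for the local player.
; On BeginPlay it takes player 0's controlled pawn, spawns a BP_FollowCamera at that pawn's transform and adds the pawn to the camera's follow targets.
; It then casts the pawn to BP_TipsyCharacter and hands it the new camera through AssignCamera.
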(event `self.ReceiveBeginPlay`
  (bind _returnvalue (`Controller.K2_GetPawn` (`GameplayStatics.GetPlayerController` 0)))
  (bind _returnvalue_2 (`self.SetupCamera` _returnvalue))
  (bind _asbp_tipsy_character (cast `/Game/TipsyTemplar/Blueprints/Characters/Templar/BP_TipsyCharacter` _returnvalue))
  (`/Game/TipsyTemplar/Blueprints/Characters/Templar/BP_TipsyCharacter.AssignCamera` _asbp_tipsy_character _returnvalue_2))

(fn `SetupCamera`
  (params (FollowTarget :type "Actor Object Reference"))
  (returns (ReturnValue :type "/Game/TipsyTemplar/Blueprints/Actors/BP_FollowCamera Object Reference"))
  (bind _returnvalue (`|SpawnActorFromClass` "/Game/TipsyTemplar/Blueprints/Actors/BP_FollowCamera.BP_FollowCamera_C" (`self.GetTransform` FollowTarget) "Undefined" "MultiplyWithRoot" null null))
  (bind _output_get (set `self.FollowCamera` _returnvalue))
  (`KismetArrayLibrary.Array_Add` (`/Game/TipsyTemplar/Blueprints/Actors/BP_FollowCamera.FollowTargets` _output_get) (`local.FollowTarget`))
  (return _returnvalue))

(fn `UserConstructionScript`)