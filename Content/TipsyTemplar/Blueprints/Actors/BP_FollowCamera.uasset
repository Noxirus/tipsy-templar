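; BP_FollowCamera is a camera actor that follows a group of targets from a fixed angle and offset.
; It sets its rotation to FollowRotation once on BeginPlay.
; Each tick it averages the FollowTargets locations into a midpoint, adds ViewOffset, and uses VInterpTo at CameraLerpSpeed to move smoothly toward that point.
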(event `self.ReceiveBeginPlay`
  (`self.K2_SetActorRotation` (`self.FollowRotation`)))

(event `self.ReceiveTick`
  (params (DeltaSeconds :type "Float (single-precision)"))
  (`self.LerpToTarget` DeltaSeconds))

(fn `CalculateLerpPosition`
  (params (DeltaTime :type "Float (double-precision)"))
  (returns (ReturnLocation :type "Vector Structure"))
  (return (`KismetMathLibrary.VInterpTo` (`self.K2_GetActorLocation`) (+ (`self.GroupMidPoint`) (`self.ViewOffset`)) (`local.DeltaTime`) (`self.CameraLerpSpeed`))))

(fn `GroupMidPoint`
  (returns (MidPoint :type "Vector Structure"))
  (locals (VectorSum :type "Vector Structure"))
  (for _array_element (`self.FollowTargets`)
    (set `local.VectorSum` (+ (`self.K2_GetActorLocation` _array_element) (`local.VectorSum`))))
  (return (/ (`local.VectorSum`) (`KismetArrayLibrary.Array_Length` (`self.FollowTargets`)))))

(fn `LerpToTarget`
  (params (DeltaTime :type "Float (double-precision)"))
  (`self.K2_SetActorLocation` (`self.CalculateLerpPosition` DeltaTime)))

(fn `UserConstructionScript`)